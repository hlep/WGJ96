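; BP_RoadLane is a road lane that spawns BP_Car actors and sets their max-speed modifier by its RoadSpeed tier.
; The construction script builds a straight spline from RoadLength and lays tier-colored spline meshes along it, with Yellow reusing the green material.
; When spawning is enabled, a looping timer plus random delay spawns cars at SpawnLocation; key 8 also spawns one.
; Cars overlapping the SpeedModifier component receive the tier's value through ModifyMaxSpeed.
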(event OnComponentBeginOverlap(SpeedModifier)
  (params (OverlappedComponent :type Primitive%20Component%20Object%20Reference) (OtherActor :type Actor%20Object%20Reference) (OtherComp :type Primitive%20Component%20Object%20Reference) (OtherBodyIndex :type Integer) (bFromSweep :type Boolean) (SweepResult :type Hit%20Result%20Structure%20%28by%20ref%29))
  (bind _asbp_car (Utilities|Casting|CastToBP_Car OtherActor))
  (Class|Car|ModifyMaxSpeed _asbp_car (Utilities|Select :Index (Variables|Default|GetRoadSpeed) :RE_Green 1.0 :RE_Yellow 1.5 :RE_Red 2.0)))

(event Custom|CarSpawnEvent
  (Utilities|FlowControl|Delay (Math|Random|RandomFloatinRange 0.0 1.0))
  (CallFunction|SpawnCar))

(event EventBeginPlay
  (Input|EnableInput (Game|GetPlayerController 0))
  (if (Variables|Default|GetbIsSpawning)
    (Utilities|Time|SetTimerbyEvent (delegate Custom|CarSpawnEvent) (Variables|Default|GetSpawnSpeed) true)))

(event Collision|EventActorBeginOverlap
  (params (OtherActor :type Actor%20Object%20Reference)))

(event EventTick
  (params (DeltaSeconds :type Float%20%28single-precision%29)))

(event Input|KeyboardEvents|8
  (params (Key :type Key%20Structure))
  (:Pressed
    (CallFunction|SpawnCar)))

(fn ConstructionScript
  (bind _spline (Variables|Default|GetSpline))
  (bind _splinepoints (LocalVariables|GetSplinePoints))
  (for _index (range 0 (Math|Float|Truncate (+ (/ (Variables|Default|GetRoadLength) 254.0) 1.0)))
    (Utilities|Array|Add _splinepoints (Math|Vector|MakeVector (* _index 254.0) 0.0 0.0)))
  (Spline|SetSplinePoints (Variables|Default|GetSpline) _splinepoints "Local" true)
  (for _index_2 (range 0 (- (Spline|GetNumberOfSplinePoints (Variables|Default|GetSpline)) 2))
    (bind _returnvalue (AddComponent|AddSplineMeshComponent true))
    (Rendering|Material|SetMaterial _returnvalue 0 (Utilities|Select :Index (Variables|Default|GetRoadSpeed) :RE_Green "/Game/RoadLane/RoadBaseGreen.RoadBaseGreen" :RE_Yellow "/Game/RoadLane/RoadBaseGreen.RoadBaseGreen" :RE_Red "/Game/RoadLane/RoadBaseRed.RoadBaseRed"))
    (Transformation|AttachComponentToComponent _returnvalue (Variables|Default|GetRoadMesh) "None" "KeepRelative" "KeepRelative" "KeepRelative" true)
    (SplineMesh|SetStartandEnd _returnvalue (.Location (Spline|GetLocationandTangentatSplinePoint _spline _index_2 "Local")) (.Tangent (Spline|GetLocationandTangentatSplinePoint _spline _index_2 "Local")) (.Location (Spline|GetLocationandTangentatSplinePoint _spline (+ _index_2 1) "Local")) (.Tangent (Spline|GetLocationandTangentatSplinePoint _spline (+ _index_2 1) "Local")) true :!class /Script/Engine.SplineMeshComponent)))

(fn SpawnCar
  (bind _spawnlocation (Variables|Default|GetSpawnLocation))
  (Game|SpawnActorfromClass "/Game/BP_Car.BP_Car_C" (Math|Transform|MakeTransform (Transformation|GetWorldLocation _spawnlocation) (Transformation|GetWorldRotation _spawnlocation) "1,1,1") "AdjustIfPossibleButDontSpawnIfColliding" 0 0))