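; BP_Car is a vehicle actor whose static mesh is picked by car class and whose physics constraint is released when hit.
; The construction script sets CarMesh by selecting on CarClass, drawing a random entry from the Car mesh list, which holds only one mesh.
; The Bus and Truck options are left empty.
; A component hit on CarMesh sets its constraint mode to None; BeginPlay and Tick are empty.
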(event OnComponentHit(CarMesh)
  (params (HitComponent :type Primitive%20Component%20Object%20Reference) (OtherActor :type Actor%20Object%20Reference) (OtherComp :type Primitive%20Component%20Object%20Reference) (NormalImpulse :type Vector :default "0, 0, 0") (Hit :type Hit%20Result%20Structure%20%28by%20ref%29))
  (Class|PrimitiveComponent|SetConstraintMode (Variables|Default|GetCarMesh) "None"))

(event EventBeginPlay)

(event Collision|EventActorBeginOverlap
  (params (OtherActor :type Actor%20Object%20Reference)))

(event EventTick
  (params (DeltaSeconds :type Float%20%28single-precision%29)))

(fn ConstructionScript
  (bind _array (Utilities|Array|MakeArray "/Game/FixedCars/FixedCars_CAR_01.FixedCars_CAR_01"))
  (Components|StaticMesh|SetStaticMesh (Variables|Default|GetCarMesh) (Utilities|Select :Index (Variables|Default|GetCarClass) :CE_Car (Utilities|Array|Get(acopy) _array (Math|Random|RandomIntegerinRange 0 (- (Utilities|Array|Length _array) 1))) :CE_Bus 0 :CE_Truck 0)))