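; BP_TrafficLIght is a clickable traffic light that toggles a stop line and counts cars.
; Clicking ClickPlane alternates the texture UVs and switches StopLine between no collision and query-only collision via a FlipFlop.
; A BP_Car overlapping StopPlane with IsCounted false triggers a click sound and the CarCounted dispatcher.
; The overlap writes IsCounted back to false, so this Blueprint never marks a car as counted.
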(event OnComponentBeginOverlap(StopPlane)
  (params (OverlappedComponent :type Primitive%20Component%20Object%20Reference) (OtherActor :type Actor%20Object%20Reference) (OtherComp :type Primitive%20Component%20Object%20Reference) (OtherBodyIndex :type Integer) (bFromSweep :type Boolean) (SweepResult :type Hit%20Result%20Structure%20%28by%20ref%29))
  (bind _asbp_car (Utilities|Casting|CastToBP_Car OtherActor))
  (if (not (Variables|/Script/WGJ96.Car|GetbIsCounted _asbp_car))
    (Variables|/Script/WGJ96.Car|SetbIsCounted _asbp_car false)
    (Audio|PlaySound2D "/Engine/VREditor/Sounds/VR_click1.VR_click1" 1.0 1.0 0.0 0 0)
    (Default|CallCarCounted)))

(event OnClicked(ClickPlane)
  (params (TouchedComponent :type Primitive%20Component%20Object%20Reference) (ButtonPressed :type Key%20Structure))
  (bind _texture (Variables|Default|GetTexture))
  (bind _stopline (Variables|Default|GetStopLine))
  (Utilities|FlowControl|FlipFlop
    (:A
      (Class|BillboardComponent|SetUV _texture 71 71)
      (Collision|SetCollisionEnabled _stopline "NoCollision"))
    (:B
      (Class|BillboardComponent|SetUV _texture 0 71)
      (Collision|SetCollisionEnabled _stopline "QueryOnly"))))

(event EventBeginPlay)

(event Collision|EventActorBeginOverlap
  (params (OtherActor :type Actor%20Object%20Reference)))

(event EventTick
  (params (DeltaSeconds :type Float%20%28single-precision%29)))

(fn ConstructionScript)