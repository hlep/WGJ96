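; BP_RoadPart is a straight road segment actor that periodically spawns BP_Car traffic.
; Its construction script lays evenly spaced spline points along local X to cover RoadLength, then builds spline mesh components between them under RoadMesh.
; A looping timer at SpawnSpeed calls SpawnCar, which randomly offsets each car left or right of SpawnLocation.
; Input is enabled so the 8 key also spawns a car.
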(event Custom|CarSpawnEvent
  (CallFunction|SpawnCar))

(event EventBeginPlay
  (Input|EnableInput (Game|GetPlayerController 0))
  (Utilities|Time|SetTimerbyEvent (delegate Custom|CarSpawnEvent) (Variables|Default|GetSpawnSpeed) true))

(event Collision|EventActorBeginOverlap
  (params (OtherActor :type Actor%20Object%20Reference)))

(event EventTick
  (params (DeltaSeconds :type Float%20%28single-precision%29)))

(event Input|KeyboardEvents|8
  (params (Key :type Key%20Structure))
  (:Pressed
    (CallFunction|SpawnCar)))

(fn ConstructionScript
  (bind _spline (Variables|Default|GetSpline))
  (bind _splinepoints (LocalVariables|GetSplinePoints))
  (for _index (range 0 (Math|Float|Truncate (+ (/ (Variables|Default|GetRoadLength) 5e+02) 1.0)))
    (Utilities|Array|Add _splinepoints (Math|Vector|MakeVector (* _index 5e+02) 0.0 0.0)))
  (Spline|SetSplinePoints (Variables|Default|GetSpline) _splinepoints "Local" true)
  (for _index_2 (range 0 (- (Spline|GetNumberOfSplinePoints (Variables|Default|GetSpline)) 2))
    (bind _returnvalue (AddComponent|AddSplineMeshComponent true))
    (Transformation|AttachComponentToComponent _returnvalue (Variables|Default|GetRoadMesh) "None" "KeepRelative" "KeepRelative" "KeepRelative" true)
    (SplineMesh|SetStartandEnd _returnvalue (.Location (Spline|GetLocationandTangentatSplinePoint _spline _index_2 "Local")) (.Tangent (Spline|GetLocationandTangentatSplinePoint _spline _index_2 "Local")) (.Location (Spline|GetLocationandTangentatSplinePoint _spline (+ _index_2 1) "Local")) (.Tangent (Spline|GetLocationandTangentatSplinePoint _spline (+ _index_2 1) "Local")) true :!class /Script/Engine.SplineMeshComponent)))

(fn SpawnCar
  (bind _spawnlocation (Variables|Default|GetSpawnLocation))
  (Game|SpawnActorfromClass "/Game/BP_Car.BP_Car_C" (Math|Transform|MakeTransform (+ (Transformation|GetWorldLocation _spawnlocation) (* (Transformation|GetActorRightVector) (Math|Conversions|ToVector(Float) (select (Math|Random|RandomBool) -3e+01 3e+01)))) (Transformation|GetWorldRotation _spawnlocation) "1,1,1") "Undefined" 0 0))